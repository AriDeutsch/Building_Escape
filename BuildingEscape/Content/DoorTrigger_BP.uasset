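; DoorTrigger_BP animates a door opening and closing in response to open and close requests from its OpenDoor component.
; The DoorSwing timeline plays forward or in reverse, with its play rate derived from the component's swing time.
; Its curve blends the referenced door actor's rotation between the component's closed and opened configurations.
; A Lock Sound event track on the timeline plays the lock sound at the door's location.
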(event OpenRequest(OpenDoor)
  (bind _opendoor (Variables|Default|GetOpenDoor))
  (Components|Timeline|SetPlayRate (Variables|Default|GetDoorSwing) (/ 1.0 (Variables|/Script/BuildingEscape.OpenDoor|GetDoorSwingTime (Variables|Default|GetOpenDoor))))
  (bind _doorswing (Timeline|DoorSwing Play)
    (:Update
      (Transformation|SetActorRotation (Variables|/Script/BuildingEscape.OpenDoor|GetDoor _opendoor) (Math|Rotator|Lerp(Rotator) (Variables|/Script/BuildingEscape.OpenDoor|GetClosedConfig _opendoor) (Variables|/Script/BuildingEscape.OpenDoor|GetOpenedConfig _opendoor) _doorswing)))
    (:Lock%20Sound
      (Audio|PlaySoundatLocation "/Game/Audio/door-lock.door-lock" (Transformation|GetActorLocation (Variables|/Script/BuildingEscape.OpenDoor|GetDoor (Variables|Default|GetOpenDoor)))))))

(event CloseRequest(OpenDoor)
  (bind _opendoor (Variables|Default|GetOpenDoor))
  (Components|Timeline|SetPlayRate (Variables|Default|GetDoorSwing) (/ 1.0 (Variables|/Script/BuildingEscape.OpenDoor|GetDoorSwingTime (Variables|Default|GetOpenDoor))))
  (bind _doorswing (Timeline|DoorSwing Reverse)
    (:Update
      (Transformation|SetActorRotation (Variables|/Script/BuildingEscape.OpenDoor|GetDoor _opendoor) (Math|Rotator|Lerp(Rotator) (Variables|/Script/BuildingEscape.OpenDoor|GetClosedConfig _opendoor) (Variables|/Script/BuildingEscape.OpenDoor|GetOpenedConfig _opendoor) _doorswing)))
    (:Lock%20Sound
      (Audio|PlaySoundatLocation "/Game/Audio/door-lock.door-lock" (Transformation|GetActorLocation (Variables|/Script/BuildingEscape.OpenDoor|GetDoor (Variables|Default|GetOpenDoor)))))))

(fn ConstructionScript)